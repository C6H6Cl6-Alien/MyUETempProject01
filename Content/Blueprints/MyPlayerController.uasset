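; Player controller that sets up the in-game HUD and handles save-and-quit for each level.
; On BeginPlay it increments the game instance's passed level count, adds the UI_Game widget and snapshots score, prior level count, buff level and level name into a new save object.
; Pressing Q writes that level-start snapshot to a slot, shows the result on the widget, then opens the main menu after a short delay, even if saving fails.
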(event `self.ReceiveBeginPlay`
  (bind _gameinstance (`self.GameInstance`))
  (`|ExecutionSequence`
    (:`then_0`
      (bind _asmy_game_instance (cast `MyGameInstance` (`GameplayStatics.GetGameInstance`)))
      (bind _output_get (set `self.GameInstance` _asmy_game_instance))
      (bind _result (`/Engine/EditorBlueprintResources/StandardMacros.IncrementInt` (`MyGameInstance.PassedLevelCount` _output_get))
        (:`  `
          (set `MyGameInstance.PassedLevelCount` _result _output_get))))
    (:`then_1`
      (bind _returnvalue (`|CreateWidget` "/Game/Blueprints/UI_Game.UI_Game_C"))
      (bind _output_get_2 (set `self.Widget` _returnvalue))
      (`UserWidget.AddToViewport` _output_get_2 0))
    (:`then_2`
      (bind _returnvalue_2 (`GameplayStatics.CreateSaveGameObject` "/Script/TempProject01.MySaveGame"))
      (bind _output_get_3 (set `self.SaveGame` _returnvalue_2))
      (set `MySaveGame.SavedScore` (`MyGameInstance.TotalScore` _gameinstance) _output_get_3)
      (set `MySaveGame.SavedLevelCount` (- (`MyGameInstance.PassedLevelCount` _gameinstance) 1) _output_get_3)
      (set `MySaveGame.SavedBuffLevel` (`MyGameInstance.BuffLevel` _gameinstance) _output_get_3)
      (bind _returnvalue_3 (`GameplayStatics.GetCurrentLevelName` true))
      (set `MySaveGame.SavedLevelName` (`KismetStringLibrary.Conv_StringToName` _returnvalue_3) _output_get_3))))

(event `Key|Q`
  (params (Key :type "Key Structure"))
  (bind _widget (`self.Widget`))
  (:`Pressed`
    (bind _returnvalue (`GameplayStatics.SaveGameToSlot` (`self.SaveGame`) "A"))
    (if _returnvalue
      (set `/Game/Blueprints/UI_Game.NoticeString` "Game has been saved and will be quitted soon..." _widget)
      (else
        (set `/Game/Blueprints/UI_Game.NoticeString` "Failed to save the game! The game will be quitted without saving..." _widget)))
    (`KismetSystemLibrary.Delay` 1.0)
    (`GameplayStatics.OpenLevel` "Level_MainMenu")))

(fn `UserConstructionScript`)